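; BP_MosterSpawner is a spawner actor that spawns monsters up to the GameMode's target kill count.
; On BeginPlay it gathers attached actors as spawn points, binds to the game-start event and reads TargetKills.
; After a start delay, a self-rearming timer spawns MonsterClass at a random point, retrying failed spawns.
; The chain ends when either the spawn total or the existing monster count reaches the target.
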(event Custom|StartSpawning
  ;[0.15 0.15 0.15 0.5] 몬스터 생성
  (Utilities|Time|SetTimerbyEvent (delegate Custom|SpawnMonster) 3.0))

(event Custom|SpawnMonster
  ;[0.15 0.15 0.15 0.5] 몬스터 생성
  (bind _outactors (Actor|GetAllActorsOfClass (Variables|Default|GetMonsterClass)))
  (if (< (Utilities|Array|Length _outactors) (Variables|Default|GetTargetSpawnCount))
    (bind _returnvalue (Game|SpawnActorfromClass (Variables|Default|GetMonsterClass) (Transformation|GetActorTransform (.OutItem (Utilities|Array|Random (Variables|Default|GetSpawnPoints)))) "Undefined" "MultiplyWithRoot" 0 0))
    (Utilities|IsValid _returnvalue
      (:Is%20Valid
        (bind _result (Math|Integer|IncrementInt (Variables|Default|GetSpawnCount))
          (:%20%20
            (if (< _result (Variables|Default|GetTargetSpawnCount))
              (CallFunction|StartSpawning)))))
      (:Is%20Not%20Valid
        (CallFunction|StartSpawning)))))

(event Custom|GameStart
  (Utilities|FlowControl|Delay (Variables|Default|GetGameStartWaitTime))
  (CallFunction|StartSpawning))

(event EventBeginPlay
  (bind _output_get (Variables|Default|SetSpawnPoints (Actor|GetAttachedActors true false)))
  (if (> (Utilities|Array|Length _output_get) 0)
    (bind _asbp_game_mode (Utilities|Casting|CastToBP_GameMode (Game|GetGameMode)))
    (EventDispatchers|BindEventtoOnGameStart _asbp_game_mode (delegate Custom|GameStart))
    (Variables|Default|SetTargetSpawnCount (Variables|/Game/Blueprints/Components/BP_GameMode.BP_GameMode_C|GetTargetKills _asbp_game_mode))))

(fn ConstructionScript)