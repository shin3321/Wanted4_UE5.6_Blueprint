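; Bear enemy monster that runs a Locomotion, Chase, Attack and Dead state machine, mirrored to its AI Blackboard.
; AI perception of a living player starts Chase; distance or player death returns it to Locomotion.
; MonsterData level stats set health, damage, defence and speeds, while BPHPController drives the HP bar and death.
; Attack-check events toggle the damage collision, and timelines drive material hit flash and death dissolve before destruction.
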(event OnComponentBeginOverlap(AttackCollision)
  (params (OverlappedComponent :type Primitive%20Component%20Object%20Reference) (OtherActor :type Actor%20Object%20Reference) (OtherComp :type Primitive%20Component%20Object%20Reference) (OtherBodyIndex :type Integer) (bFromSweep :type Boolean) (SweepResult :type Hit%20Result%20Structure%20%28by%20ref%29))
  ;[0.15 0.15 0.15 0.5] 플레이어에 대미지 전달
  (Game|Damage|ApplyDamage OtherActor (Variables|Default|GetDamage) (Pawn|GetController) self))

(event OnTargetPerceptionUpdated(AIPerception)
  (params (Actor :type Actor%20Object%20Reference) (Stimulus :type AI%20Stimulus%20Structure))
  ;[0.07217 0.1446 0.15 0.5] Ai Perception
  (if (.bSuccessfullySensed (Utilities|Struct|BreakAIStimulus Stimulus))
    (if (Utilities|Enum|Equal(Enum) (Variables|Default|GetState_BP) "NewEnumerator0")
      (if (Actor|ActorHasTag Actor "Player")
        (AI|Components|Blackboard|SetValueasObject (Variables|/Script/AIModule.AIController|GetBlackboard (AI|GetAIController self)) (Variables|Default|GetTargetPlayerKey) Actor)
        (bind _asbp_charactor_2 (Utilities|Casting|CastToBP_Charactor2 Actor))
        (if (not (Utilities|Enum|Equal(Enum) (Variables|/Game/Blueprints/Charactor/BP_Charactor2.BP_Charactor2_C|GetState_BP _asbp_charactor_2) "NewEnumerator2"))
          (CallFunction|UpdateState "NewEnumerator1"))))))

(event Custom|ReceiveOnDead
  (bind _mesh (Variables|Character|GetMesh))
  ;[0.09853 0.0875 0.15 0.5] 죽음 이벤트에 바인딩
  (CallFunction|UpdateState "NewEnumerator3")
  (Collision|SetCollisionEnabled (Variables|Collision|GetCapsuleComponent) "NoCollision")
  (Utilities|FlowControl|Delay 3.0)
  (bind _dissolve (Timeline|DeathEffect Play)
    (:Update
      (Rendering|Material|SetScalarParameterValueonMaterials _mesh "Dissolve" _dissolve)
      (Rendering|Material|SetScalarParameterValueonMaterials _mesh "Hitvalue" 0.0))
    (:Finished
      (Actor|DestroyActor))))

(event Custom|UpdateState
  (params (NewState :type EBearState%20Enum :default "NewEnumerator0"))
  (bind _monsterdata (Variables|Default|GetMonsterData))
  (bind _charactermovement (Variables|Character|GetCharacterMovement))
  (bind _currentleveldata (Default|GetCurrentLevelData _monsterdata))
  ;[0.15 0.15 0.15 0.5] 몬스터 상태 변경 이벤트
  (if (Utilities|Enum|NotEqual(Enum) (Variables|Default|GetState_BP) "NewEnumerator3")
    (bind _output_get (Variables|Default|SetState_BP NewState))
    (AI|Components|Blackboard|SetValueasEnum (Variables|/Script/AIModule.AIController|GetBlackboard (AI|GetAIController self)) (Variables|Default|GetStateKey) _output_get)
    (switch Utilities|FlowControl|Switch|SwitchonEBearState (Variables|Default|GetState_BP)
      (:NewEnumerator0
        (Variables|/Script/Engine.CharacterMovementComponent|SetMaxWalkSpeed _charactermovement (.walkspeed _currentleveldata)))
      (:NewEnumerator1
        (Variables|/Script/Engine.CharacterMovementComponent|SetMaxWalkSpeed _charactermovement (.chasespeed _currentleveldata)))
      (:NewEnumerator2
        (Variables|/Script/Engine.CharacterMovementComponent|SetMaxWalkSpeed _charactermovement 0.0 :!label _label))
      (:NewEnumerator3
        (goto _label)))))

(event Custom|OnAttackCheckEnd
  ;[0.5938 0.2392 0.07551 0.5] 공격 판정 시작 종료
  (Collision|SetCollisionEnabled (Variables|Default|GetAttackCollision) "NoCollision"))

(event Custom|OnAttackCheckStart
  ;[0.5938 0.2392 0.07551 0.5] 공격 판정 시작 종료
  (Collision|SetCollisionEnabled (Variables|Default|GetAttackCollision) "QueryOnly"))

(event Custom|ReceiveOnHpChanged
  (params (HealthPower :type Float%20%28double-precision%29) (MaxHealthPower :type Float%20%28double-precision%29))
  ;[0.15 0.15 0.15 0.5] HPBar 업데이트
  (bind _aswbp_bear_hp (Utilities|Casting|CastToWBP_BearHP (UserInterface|GetUserWidgetObject (Variables|Default|GetHPBar))))
  (Default|UpdateHpPercent _aswbp_bear_hp (/ HealthPower MaxHealthPower)))

(event Game|Damage|EventAnyDamage
  (params (Damage :type Float%20%28single-precision%29) (DamageType :type Damage%20Type%20Object%20Reference) (InstigatedBy :type Controller%20Object%20Reference) (DamageCauser :type Actor%20Object%20Reference))
  ;[0.15 0.15 0.15 0.5] 데미지
  (CallFunction|TurntoTarget DamageCauser)
  (Default|ReceiveDamage (Variables|Default|GetBP_HPController) (- (.Defence (Utilities|Struct|BreakBP_MonsterLevelData (Default|GetCurrentLevelData (Variables|Default|GetMonsterData)))) Damage))
  ;;[0.15 0.15 0.15 0.5] 맞았을 때 피격 효과
  (bind _hitvalue (Timeline|Timeline PlayFromStart)
    (:Update
      (Rendering|Material|SetScalarParameterValueonMaterials (Variables|Character|GetMesh) "HitValue" _hitvalue))))

(event EventBeginPlay
  (bind _monsterdata (Variables|Default|GetMonsterData))
  (bind _currentleveldata (Default|GetCurrentLevelData _monsterdata))
  (bind (_attack _defence _walkspeed _chasespeed _maxhp) (Utilities|Struct|BreakBP_MonsterLevelData _currentleveldata))
  ;[0.09853 0.0875 0.15 0.5] 죽음 이벤트에 바인딩
  (EventDispatchers|BindEventtoOnDeadEvent (Variables|Default|GetBP_HPController) (delegate Custom|ReceiveOnDead))
  ;[0.4348 0.4348 1 0.5] 시작 시 공격 콜리젼 끄기
  (Collision|SetCollisionEnabled (Variables|Default|GetAttackCollision) "NoCollision")
  ;[0.15 0.15 0.15 0.5] HPBar 업데이트
  (EventDispatchers|BindEventtoOnHpChanged (Variables|Default|GetBP_HPController) (delegate Custom|ReceiveOnHpChanged))
  ;[0.15 0.15 0.15 0.5] 몬스터 레벨 데이터 가져오기
  (Default|UpdateMaxHP (Variables|Default|GetBP_HPController) _maxhp)
  (Variables|Default|SetDamage _attack))

(event EventTick
  (params (DeltaSeconds :type Float%20%28single-precision%29))
  ;[0.15 0.15 0.15 0.5] 곰 상태 감지
  (switch Utilities|FlowControl|Switch|SwitchonEBearState (Variables|Default|GetState_BP)
    (:NewEnumerator0
      (CallFunction|OnLocomation))
    (:NewEnumerator1
      (CallFunction|OnChase) ; 플레이어 위치를 받아와서 추적 처리
    )
    (:NewEnumerator2
      (CallFunction|OnAttack))
    (:NewEnumerator3
      (CallFunction|OnDead))))

(fn ConstructionScript)

(fn OnChase
  (bind _asactor (Utilities|Casting|CastToActor (AI|Components|Blackboard|GetValueasObject (Variables|/Script/AIModule.AIController|GetBlackboard (AI|GetAIController self)) (Variables|Default|GetTargetPlayerKey))))
  (if (> (Math|Vector|Distance(Vector) (Transformation|GetActorLocation _asactor) (Transformation|GetActorLocation)) 4e+02)
    (CallFunction|UpdateState "NewEnumerator0")))

(fn OnLocomation)

(fn OnAttack
  (bind _asbp_charactor_2 (Utilities|Casting|CastToBP_Charactor2 (AI|Components|Blackboard|GetValueasObject (Variables|/Script/AIModule.AIController|GetBlackboard (AI|GetAIController self)) (Variables|Default|GetTargetPlayerKey))))
  (if (Utilities|Enum|Equal(Enum) (Variables|/Game/Blueprints/Charactor/BP_Charactor2.BP_Charactor2_C|GetState_BP _asbp_charactor_2) "NewEnumerator2")
    (CallFunction|UpdateState "NewEnumerator0")))

(fn OnDead)

(fn TurntoTarget
  (params (TargetPlayer :type Actor%20Object%20Reference))
  (switch Utilities|FlowControl|Switch|SwitchonEBearState (Variables|Default|GetState_BP)
    (:NewEnumerator0
      (Transformation|SetActorRotation self (Math|Rotator|MakeRotator 0.0 0.0 (.yaw (Math|Rotator|MakeRotfromX (- (Transformation|GetActorLocation TargetPlayer) (Transformation|GetActorLocation)))))))))